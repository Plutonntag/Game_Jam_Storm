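; BP_Camera_Character is the player camera character Blueprint, which handles pause menu input.
; IA_MenuPause toggles a BP_PauseMenu widget, switching game pause, input mode and mouse cursor visibility along with it.
; A Stat event prints the Durabilite value for debugging.
; Disconnected nodes for clearing RefCharacter and opening the BP_Menu and BP_Statistique widgets never run.
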(event Custom|Stat
  (Development|PrintString (Utilities|String|ToString(Float) (Variables|Default|GetDurabilite))))

(event Input|EnhancedActionEvents|EnhancedInputActionIA_MenuPause
  (params (ActionValue :type Boolean) (ElapsedSeconds :type Float%20%28double-precision%29) (TriggeredSeconds :type Float%20%28double-precision%29) (InputAction :type Input%20Action%20Object%20Reference :default "/Game/Migrate_Axel/TopDown/Input/Actions/IA_MenuPause.IA_MenuPause"))
  (bind _returnvalue (Game|GetPlayerController 0))
  (if (not (Variables|Default|GetIsMenuPauseOpen?))
    (Variables|Default|SetIsMenuPauseOpen? true)
    (bind _returnvalue_2 (UserInterface|CreateWidget "/Game/Migrate_Axel/UI/Pause_Menu/BP_PauseMenu.BP_PauseMenu_C" _returnvalue))
    (bind _output_get (Variables|Default|SetWidget%20Pause%20Menu _returnvalue_2))
    (UserInterface|Viewport|AddtoViewport _output_get 0)
    (Input|SetInputModeGameandUI _returnvalue (Variables|Default|GetWidget%20Pause%20Menu) "DoNotLock" true false)
    (Variables|/Script/Engine.PlayerController|SetbShowMouseCursor (Game|GetPlayerController 0) true)
    (Game|SetGamePaused true)
    (else
      (Variables|Default|SetIsMenuPauseOpen? false)
      (Widget|RemovefromParent (Variables|Default|GetWidget%20Pause%20Menu))
      (Game|SetGamePaused false)
      (Input|SetInputModeGameOnly _returnvalue false)
      (Variables|/Script/Engine.PlayerController|SetbShowMouseCursor (Game|GetPlayerController 0) false))))

(event EventBeginPlay)

(event Collision|EventActorBeginOverlap
  (params (OtherActor :type Actor%20Object%20Reference)))

(event EventTick
  (params (DeltaSeconds :type Float%20%28single-precision%29)))

(fn ConstructionScript)