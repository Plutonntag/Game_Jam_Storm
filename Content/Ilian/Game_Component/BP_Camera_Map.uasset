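; BP_Camera_Map is a map object whose sphere detects tornado hits and damages the player character's PV, Impermeable and Durabilite stats.
; On overlap it destroys the tornado and sets losses from its type, applying them immediately for known types.
; It then adjusts losses through one-shot protection flags and penalties for non-negative Impermeable or Durabilite, and subtracts them again.
; BloqueCroc derives the durability loss from the waterproofing loss.
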(event OnComponentBeginOverlap(Sphere)
  (params (OverlappedComponent :type Primitive%20Component%20Object%20Reference) (OtherActor :type Actor%20Object%20Reference) (OtherComp :type Primitive%20Component%20Object%20Reference) (OtherBodyIndex :type Integer) (bFromSweep :type Boolean) (SweepResult :type Hit%20Result%20Structure%20%28by%20ref%29))
  (bind _asbp_tornade (Utilities|Casting|CastToBP_Tornade OtherActor))
  (Actor|DestroyActor _asbp_tornade)
  (CallFunction|TypeTornade)
  (CallFunction|Bonus)
  (CallFunction|Malus)
  (CallFunction|BaisseStatistique))

(event Custom|Baisse_Statistique
  (bind _ref_character (Variables|Default|GetRef%20character))
  (Variables|/Game/Ilian/Game_Component/BP_Camera_Character.BP_Camera_Character_C|SetPV _ref_character (- (Variables|/Game/Ilian/Game_Component/BP_Camera_Character.BP_Camera_Character_C|GetPV _ref_character) (Variables|Default|GetPV_lost)))
  (Variables|/Game/Ilian/Game_Component/BP_Camera_Character.BP_Camera_Character_C|SetImpermeable _ref_character (- (Variables|/Game/Ilian/Game_Component/BP_Camera_Character.BP_Camera_Character_C|GetImpermeable _ref_character) (Variables|Default|GetImper_Lost)))
  (Variables|/Game/Ilian/Game_Component/BP_Camera_Character.BP_Camera_Character_C|SetDurabilite _ref_character (- (Variables|/Game/Ilian/Game_Component/BP_Camera_Character.BP_Camera_Character_C|GetDurabilite _ref_character) (Variables|Default|GetDura_Lost))))

(event Custom|Type_Tornade
  (Utilities|FlowControl|Sequence
    (:then_0
      (if (== (.typetornade (Variables|/Game/Ilian/Game_Component/BP_Tornade.BP_Tornade_C|GetStructure (stale OnComponentBeginOverlap(Sphere) _asbp_tornade))) 1.0)
        (Variables|Default|SetPV_lost 1.0)
        (Variables|Default|SetImper_Lost 2.0)
        (Variables|Default|SetDura_Lost 1.0)
        (CallFunction|BaisseStatistique :!label _label)))
    (:then_1
      (if (== (.typetornade (Variables|/Game/Ilian/Game_Component/BP_Tornade.BP_Tornade_C|GetStructure (stale OnComponentBeginOverlap(Sphere) _asbp_tornade))) 2.0)
        (Variables|Default|SetPV_lost 3.0)
        (Variables|Default|SetImper_Lost 2.0)
        (Variables|Default|SetDura_Lost 2.0)
        (goto _label)))
    (:then_2
      (if (== (.typetornade (Variables|/Game/Ilian/Game_Component/BP_Tornade.BP_Tornade_C|GetStructure (stale OnComponentBeginOverlap(Sphere) _asbp_tornade))) 3.0)
        (Variables|Default|SetPV_lost 2.0)
        (Variables|Default|SetImper_Lost 2.0)
        (Variables|Default|SetDura_Lost 3.0)
        (goto _label)))))

(event Custom|Bonus
  ;[0.15 0.15 0.15 0.5] Bonus
  (Utilities|FlowControl|Sequence
    (:then_0
      (if (Variables|/Game/Ilian/Game_Component/BP_Camera_Character.BP_Camera_Character_C|GetAnti_Feu (Variables|Default|GetRef%20character))
        (Variables|Default|SetPV_lost (- (Variables|Default|GetPV_lost) 1.0))
        (Variables|/Game/Ilian/Game_Component/BP_Camera_Character.BP_Camera_Character_C|SetAnti_Feu (Variables|Default|GetRef%20character) false)))
    (:then_1
      (if (Variables|/Game/Ilian/Game_Component/BP_Camera_Character.BP_Camera_Character_C|GetBloque_croc (Variables|Default|GetRef%20character))
        (Variables|Default|SetDura_Lost (- (Variables|Default|GetImper_Lost) 1.0))
        (Variables|/Game/Ilian/Game_Component/BP_Camera_Character.BP_Camera_Character_C|SetBloque_croc (Variables|Default|GetRef%20character) false)))
    (:then_2
      (if (Variables|/Game/Ilian/Game_Component/BP_Camera_Character.BP_Camera_Character_C|GetAnti_rouille (Variables|Default|GetRef%20character))
        (Variables|Default|SetDura_Lost (- (Variables|Default|GetDura_Lost) 1.0))
        (Variables|/Game/Ilian/Game_Component/BP_Camera_Character.BP_Camera_Character_C|SetAnti_rouille (Variables|Default|GetRef%20character) false)))))

(event Custom|Malus
  ;[0.15 0.15 0.15 0.5] Malus
  (Utilities|FlowControl|Sequence
    (:then_0
      (if (<= 0.0 (Variables|/Game/Ilian/Game_Component/BP_Camera_Character.BP_Camera_Character_C|GetImpermeable (Variables|Default|GetRef%20character)))
        (Variables|Default|SetPV_lost (+ (Variables|Default|GetPV_lost) 1.0))))
    (:then_1
      (if (<= 0.0 (Variables|/Game/Ilian/Game_Component/BP_Camera_Character.BP_Camera_Character_C|GetDurabilite (Variables|Default|GetRef%20character)))
        (Variables|Default|SetPV_lost (+ (Variables|Default|GetPV_lost) 1.0))))))

(event EventBeginPlay
  (bind _asbp_camera_character (Utilities|Casting|CastToBP_Camera_Character (Game|Player|GetPlayerPawn 0)))
  (Variables|Default|SetRef%20character _asbp_camera_character))

(fn ConstructionScript)