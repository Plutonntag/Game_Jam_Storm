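; BP_Tornade is a tornado actor that launches itself in a random horizontal direction on BeginPlay and increments the tornado count on BP_Camera_Character.
; AddForce on Tornade uses random X/Y magnitudes with random signs.
; Three sequenced checks can set Image to a water, fire or shark material.
; Each check re-rolls its random integer, so the look can differ from the stored TypeTornade or stay default.
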(event EventBeginPlay
  (bind _returnvalue (Math|Random|RandomIntegerinRange 1 3))
  (bind _returnvalue_2 (Math|Random|RandomFloatinRange -1.5e+03 -2.5e+03))
  (bind _returnvalue_3 (Math|Random|RandomBool))
  (bind _returnvalue_4 (Math|Random|RandomBool))
  (bind _returnvalue_5 (Math|Random|RandomFloatinRange 1.5e+03 2.5e+03))
  (bind _returnvalue_6 (Math|Random|RandomFloatinRange 1.5e+03 2.5e+03))
  (bind _returnvalue_7 (Math|Random|RandomFloatinRange -1.5e+03 -2.5e+03))
  (bind _returnvalue_8 (select _returnvalue_4 _returnvalue_2 _returnvalue_5))
  (bind _returnvalue_9 (select _returnvalue_3 _returnvalue_7 _returnvalue_6))
  (bind _asbp_camera_character (Utilities|Casting|CastToBP_Camera_Character (Game|Player|GetPlayerPawn 0)))
  (Variables|Default|SetRef%20character _asbp_camera_character)
  (Variables|Default|SetX_Random _returnvalue_9)
  (Variables|Default|SetY_random _returnvalue_8)
  ;[0.15 0.15 0.15 0.5] AddForce pour le mouvement
  (Physics|AddForce (Variables|Default|GetTornade) (Math|Vector|MakeVector _returnvalue_9 _returnvalue_8 0.0) "None" false)
  (Variables|/Game/Ilian/Game_Component/BP_Camera_Character.BP_Camera_Character_C|SetNumber_Tornade (Variables|Default|GetRef%20character) (+ (Variables|/Game/Ilian/Game_Component/BP_Camera_Character.BP_Camera_Character_C|GetNumber_Tornade (Variables|Default|GetRef%20character)) 1))
  (Variables|Default|SetType_Tornade (Utilities|Struct|MakeType_Tornade _returnvalue))
  (Utilities|FlowControl|Sequence
    (:then_0
      (if (== _returnvalue 1.0)
        (Rendering|Material|SetMaterial (Variables|Default|GetImage) 0 "/Game/Ilian/Game_Component/Material/MT_Tornade_Eau.MT_Tornade_Eau")))
    (:then_1
      (if (== _returnvalue 2.0)
        (Rendering|Material|SetMaterial (Variables|Default|GetImage) 0 "/Game/Ilian/Game_Component/Material/MT_Tornade_Feu.MT_Tornade_Feu")))
    (:then_2
      (if (== _returnvalue 3.0)
        (Rendering|Material|SetMaterial (Variables|Default|GetImage) 0 "/Game/Ilian/Game_Component/Material/MT_Tornade_Requin.MT_Tornade_Requin")))))

(event Collision|EventActorBeginOverlap
  (params (OtherActor :type Actor%20Object%20Reference)))

(event EventTick
  (params (DeltaSeconds :type Float%20%28single-precision%29)))

(fn ConstructionScript)